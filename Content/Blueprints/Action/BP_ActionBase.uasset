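; BP_ActionBase is a base action that an owning component can start and stop on behalf of a stored instigator.
; Starting adds the action's type tags to the owning component and marks it running, while stopping removes them and clears that flag.
; CanStart refuses when the action is already running or the component's tag search finds its blocked action type, so active actions can block others through tags.
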(fn `CanStart`
  (returns (CanStart :type Boolean))
  (if (`self.bIsRunning`)
    (return false)
    (else
      (bind _typefound (`/Game/Blueprints/Action/AC_ActionComponent.SearchTag` (`self.OwningComponent`) (`.BlockedActionType_6_1798F4054E5C190809E4FD983B7F7232` (break `/Game/Blueprints/Action/Struct/S_Action` (`self.Properties`)))))
      (if _typefound
        (return false)
        (else
          (return true))))))

(fn `Initialize`
  (params (Instigator :type "Actor Object Reference"))
  (set `self.Instigator` Instigator))

(fn `StartAction`
  (`/Game/Blueprints/Action/AC_ActionComponent.AddActionTypes` (`self.OwningComponent`) (`.ActionTypes_5_73AEDDFB43CE7AF89455118DBE33AE3F` (break `/Game/Blueprints/Action/Struct/S_Action` (`self.Properties`))))
  (set `self.bIsRunning` true))

(fn `StopAction`
  (`/Game/Blueprints/Action/AC_ActionComponent.RemoveActionTypes` (`self.OwningComponent`) (`.ActionTypes_5_73AEDDFB43CE7AF89455118DBE33AE3F` (break `/Game/Blueprints/Action/Struct/S_Action` (`self.Properties`))))
  (set `self.bIsRunning` false))