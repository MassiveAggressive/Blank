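; Action component that keeps a list of the action types currently active on its owner.
; AddActionTypes appends incoming types without a duplicate check, and RemoveActionTypes removes the first matching entry for each type passed in.
; SearchTag reports whether any of the queried types is in the active list, stopping at the first match.
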(fn `AddActionTypes`
  (params (Array :type "Array of /Game/Blueprints/Action/ActionType/E_ActionType Enum"))
  (`KismetArrayLibrary.Array_Append` (`self.ActiveActionsTypes`) Array))

(fn `RemoveActionTypes`
  (params (Array :type "Array of /Game/Blueprints/Action/ActionType/E_ActionType Enum"))
  (bind _activeactionstypes (`self.ActiveActionsTypes`))
  (for _array_element Array
    (`KismetArrayLibrary.Array_Remove` _activeactionstypes (`KismetArrayLibrary.Array_Find` _activeactionstypes _array_element))))

(fn `SearchTag`
  (params (Array :type "Array of /Game/Blueprints/Action/ActionType/E_ActionType Enum"))
  (returns (TypeFound :type Boolean))
  (locals (TypeFoundRef :type Boolean :default false))
  (for _array_element Array
    (bind _returnvalue (!= (`KismetArrayLibrary.Array_Find` (`self.ActiveActionsTypes`) _array_element) -1))
    (if _returnvalue
      (set `local.TypeFoundRef` _returnvalue)
      (break)))
  (return (`local.TypeFoundRef`)))