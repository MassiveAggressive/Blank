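; BP_ProjectileBase is a base projectile that delivers damage on impact and destroys itself.
; When its Box component hits, it passes Damage to the other actor through BPI_HealthInterface, if implemented.
; Every hit spawns NS_Sparks at the impact point, oriented along the surface normal.
; A shared Color variable tints both the sparks and a dynamic bullet material created in the construction script.
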(event `self.Box.OnComponentHit`
  (params (HitComponent :type "PrimitiveComponent Object Reference") (OtherActor :type "Actor Object Reference") (OtherComp :type "PrimitiveComponent Object Reference") (NormalImpulse :type "Vector Structure") (Hit :type "HitResult Structure (by ref)"))
  (bind (_bblockinghit _binitialoverlap _time _distance _location _impactpoint _normal _impactnormal) (`GameplayStatics.BreakHitResult` Hit))
  (if (`KismetSystemLibrary.DoesImplementInterface` OtherActor "/Game/Blueprints/Health/BPI_HealthInterface.BPI_HealthInterface_C")
    (message `/Game/Blueprints/Health/BPI_HealthInterface.AddHealth` OtherActor "NewEnumerator1" (`self.Damage`)))
  (bind _returnvalue (`NiagaraFunctionLibrary.SpawnSystemAtLocation` "/Game/Assets/Particle/NS_Sparks.NS_Sparks" _impactpoint (`KismetMathLibrary.Conv_VectorToRotator` _impactnormal)))
  (`FXSystemComponent.SetColorParameter` _returnvalue "Color" (`self.Color`))
  (`self.K2_DestroyActor`))

(fn `UserConstructionScript`
  (bind _returnvalue (`PrimitiveComponent.CreateDynamicMaterialInstance` (`self.Mesh`) 0 "/Game/Assets/Material/MI_Bullet.MI_Bullet" "None"))
  (`MaterialInstanceDynamic.SetVectorParameterValue` _returnvalue "Color" (`self.Color`)))