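; BP_SingleWeapon is a child weapon Blueprint that fires one projectile from a single barrel.
; Its construction script adds one arrow component to the Barrels array as the muzzle.
; Shoot calls the parent logic, then spawns BP_ProjectileBase at that arrow's world transform, ignoring collisions at the spawn point.
; The functions for adding or setting barrel count and distance are empty, so they leave the single-barrel layout unchanged.
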(event `self.ReceiveBeginPlay`
  (`parent.ReceiveBeginPlay`))

(event `self.Shoot`
  (params (AffectedBySkill :type Boolean))
  (`parent.Shoot` AffectedBySkill)
  (`|SpawnActorFromClass` "/Game/Blueprints/Weapon/Projectile/BP_ProjectileBase.BP_ProjectileBase_C" (`SceneComponent.K2_GetComponentToWorld` (`|GetArrayItem` (`self.Barrels`))) "AlwaysSpawn" "OverrideRootScale" null null))

(fn `AddBarrelCount`
  (params (Delta :type Integer)))

(fn `AddBarrelDistance`
  (params (Delta :type "Float (double-precision)")))

(fn `SetBarrelCount`
  (params (Value :type Integer)))

(fn `SetBarrelDistance`
  (params (Value :type "Float (double-precision)")))

(fn `UserConstructionScript`
  (`parent.UserConstructionScript`)
  (bind _returnvalue (`AddComponent|NODE_AddArrowComponent-2`))
  (`KismetArrayLibrary.Array_Add` (`self.Barrels`) _returnvalue))