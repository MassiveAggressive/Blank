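; Shotgun weapon Blueprint, derived from a parent weapon, that fires a spread of projectiles from a single muzzle.
; Construction adds one arrow component as the barrel; BarrelCount acts as pellet count rather than physical barrels.
; Shoot calls the parent, then spawns one BP_ProjectileBase per count, each randomly yawed around world Z within ±ScatterAmount degrees.
; Count and scatter are adjustable, while barrel-distance changes are ignored or forced to zero.
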(event `self.Shoot`
  (params (AffectedBySkill :type Boolean))
  (bind _scatteramount (`self.ScatterAmount`))
  (bind _output (`|GetArrayItem` (`self.Barrels`)))
  (`parent.Shoot` AffectedBySkill)
  (for _ (range (`self.BarrelCount`))
    (`|SpawnActorFromClass` "/Game/Blueprints/Weapon/Projectile/BP_ProjectileBase.BP_ProjectileBase_C" (`KismetMathLibrary.MakeTransform` (`SceneComponent.K2_GetComponentLocation` _output) (`KismetMathLibrary.Conv_VectorToRotator` (`KismetMathLibrary.RotateAngleAxis` (`KismetMathLibrary.GetForwardVector` (`SceneComponent.K2_GetComponentRotation` _output)) (`KismetMathLibrary.RandomFloatInRange` (* _scatteramount -1.0) _scatteramount) (0.0 0.0 1.0)))) "AlwaysSpawn" "OverrideRootScale" null null)))

(fn `AddBarrelCount`
  (params (Delta :type Integer))
  (set `self.BarrelCount` (+ (`self.BarrelCount`) Delta)))

(fn `AddBarrelDistance`
  (params (Delta :type "Float (double-precision)")))

(fn `AddScatterAmount`
  (params (Delta :type "Float (double-precision)"))
  (set `self.ScatterAmount` (+ (`self.ScatterAmount`) Delta)))

(fn `SetBarrelCount`
  (params (Value :type Integer))
  (set `self.BarrelCount` Value))

(fn `SetBarrelDistance`
  (params (Value :type "Float (double-precision)"))
  (`parent.SetBarrelDistance` 0.0))

(fn `SetScatterAmount`
  (params (Value :type "Float (double-precision)"))
  (set `self.ScatterAmount` Value))

(fn `UserConstructionScript`
  (`parent.UserConstructionScript`)
  (bind _returnvalue (`AddComponent|NODE_AddArrowComponent-1`))
  (`KismetArrayLibrary.Array_Add` (`self.Barrels`) _returnvalue))