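; Base weapon Blueprint that starts auto-firing on BeginPlay and manages fire rate and a row of barrels.
; A looping timer paces shots, with Shoot calling Shooted and clearing availability; no projectile logic lives here.
; Fire-rate changes scale the remaining cooldown proportionally before restarting the timer.
; Barrel setters add or reposition arrow components evenly centered along local Y, clearing the array on count changes without destroying old components.
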(event `self.ReceiveBeginPlay`
  (`self.StartShooting`))

(event `SetShootAvailable`
  (set `self.IsShootAvailable` true)
  (if (`self.IsShooting`)
    (`self.Shoot` false)
    (else
      (`KismetSystemLibrary.K2_ClearAndInvalidateTimerHandle` (`self.ShootTimer`)))))

(event `Shoot`
  (params (AffectedBySkill :type Boolean))
  (`self.Shooted` AffectedBySkill)
  (set `self.IsShootAvailable` false))

(event `FireRateChanged`
  (bind _shoottimer (`self.ShootTimer`))
  (bind _returnvalue (`KismetSystemLibrary.K2_GetTimerRemainingTimeHandle` _shoottimer))
  (`KismetSystemLibrary.K2_ClearAndInvalidateTimerHandle` (`self.ShootTimer`))
  (`KismetSystemLibrary.Delay` (* (/ 1.0 (`self.FireRate`)) (/ _returnvalue (+ (`KismetSystemLibrary.K2_GetTimerElapsedTimeHandle` _shoottimer) _returnvalue))))
  (if (`self.IsShooting`)
    (`self.SetShootAvailable`)
    (bind _returnvalue_2 (`KismetSystemLibrary.K2_SetTimerDelegate` (`|CreateDelegate` :!event `SetShootAvailable`) (/ 1.0 (`self.FireRate`)) true))
    (set `self.ShootTimer` _returnvalue_2)))

(fn `AddBarrelCount`
  (params (Delta :type Integer))
  (bind _output_get (set `self.BarrelCount` (+ (`self.BarrelCount`) Delta)))
  (`KismetArrayLibrary.Array_Clear` (`self.Barrels`))
  (bind _returnvalue (- _output_get 1))
  (for _index (range (+ _returnvalue 1))
    (bind _returnvalue_2 (`AddComponent|NODE_AddArrowComponent-1` :`RelativeTransform` (`KismetMathLibrary.MakeTransform` (`KismetMathLibrary.MakeVector` 0.0 (- (* _index (`self.BarrelDistance`)) (/ (* _returnvalue (`self.BarrelDistance`)) 2.0))))))
    (`KismetArrayLibrary.Array_Add` (`self.Barrels`) _returnvalue_2)))

(fn `AddBarrelDistance`
  (params (Delta :type "Float (double-precision)"))
  (set `self.BarrelDistance` (+ (`self.BarrelDistance`) Delta))
  (for (_array_element _array_index) (`self.Barrels`)
    (`SceneComponent.K2_SetRelativeLocation` _array_element (`KismetMathLibrary.MakeVector` 0.0 (- (* _array_index (`self.BarrelDistance`)) (/ (* (- (`self.BarrelCount`) 1) (`self.BarrelDistance`)) 2.0))) false false)))

(fn `AddFireRate`
  (params (Delta :type "Float (double-precision)"))
  (set `self.FireRate` (+ (`self.FireRate`) Delta))
  (`self.FireRateChanged`))

(fn `SetBarrelCount`
  (params (Value :type Integer))
  (bind _output_get (set `self.BarrelCount` Value))
  (`KismetArrayLibrary.Array_Clear` (`self.Barrels`))
  (bind _returnvalue (- _output_get 1))
  (for _index (range (+ _returnvalue 1))
    (bind _returnvalue_2 (`AddComponent|NODE_AddArrowComponent-2` :`RelativeTransform` (`KismetMathLibrary.MakeTransform` (`KismetMathLibrary.MakeVector` 0.0 (- (* _index (`self.BarrelDistance`)) (/ (* _returnvalue (`self.BarrelDistance`)) 2.0))))))
    (`KismetArrayLibrary.Array_Add` (`self.Barrels`) _returnvalue_2)))

(fn `SetBarrelDistance`
  (params (Value :type "Float (double-precision)"))
  (set `self.BarrelDistance` Value)
  (for (_array_element _array_index) (`self.Barrels`)
    (`SceneComponent.K2_SetRelativeLocation` _array_element (`KismetMathLibrary.MakeVector` 0.0 (- (* _array_index (`self.BarrelDistance`)) (/ (* (- (`self.BarrelCount`) 1) (`self.BarrelDistance`)) 2.0))) false false)))

(fn `SetFireRate`
  (params (Value :type "Float (double-precision)"))
  (set `self.FireRate` Value)
  (`self.FireRateChanged`))

(fn `StartShooting`
  (set `self.IsShooting` true)
  (if (`self.IsShootAvailable`)
    (`self.Shoot` false))
  (bind _returnvalue (`KismetSystemLibrary.K2_SetTimerDelegate` (`|CreateDelegate` :!event `SetShootAvailable`) (/ 1.0 (`self.FireRate`)) true))
  (set `self.ShootTimer` _returnvalue))

(fn `StopShooting`
  (set `self.IsShooting` false))

(fn `UserConstructionScript`)