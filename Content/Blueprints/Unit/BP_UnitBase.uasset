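; BP_UnitBase is a base unit actor with a health component and a static mesh.
; It forwards add health, add max health and set max health events to the component, and destroys itself when the component fires OnDestroy.
; It exposes the mesh and a socket lookup that converts a socket type enum to the socket name and returns its world transform.
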(event `/Game/Blueprints/Health/BPI_HealthInterface.AddHealth`
  (params (AddHealthType :type "/Game/Blueprints/Health/E_AddHealthType Enum" :default "NewEnumerator0") (Value :type "Float (single-precision)"))
  (`/Game/Blueprints/Health/AC_HealthComponent.AddHealth` (`self.AC_HealthComponent`) AddHealthType Value))

(event `self.AC_HealthComponent.OnDestroy`
  (`self.K2_DestroyActor`))

(event `/Game/Blueprints/Health/BPI_HealthInterface.AddMaxHealth`
  (params (Value :type "Float (single-precision)"))
  (`/Game/Blueprints/Health/AC_HealthComponent.AddMaxHealth` (`self.AC_HealthComponent`) Value))

(event `/Game/Blueprints/Health/BPI_HealthInterface.SetMaxHealth`
  (params (Value :type "Float (single-precision)"))
  (`/Game/Blueprints/Health/AC_HealthComponent.SetMaxHealth` (`self.AC_HealthComponent`) Value))

(fn `GetMesh`
  (returns (Mesh :type "MeshComponent Object Reference"))
  (return (`self.StaticMesh`)))

(fn `GetSocket`
  (params (SocketType :type "/Game/Blueprints/Unit/SocketsEnum/E_SocketType Enum" :default "NewEnumerator0"))
  (returns (Socket :type Name) (SocketTransform :type "Transform Structure"))
  (bind _returnvalue (`KismetStringLibrary.Conv_StringToName` (`|GetEnumeratorNameAsString` SocketType)))
  (return _returnvalue (`SceneComponent.GetSocketTransform` (`self.StaticMesh`) _returnvalue "RTS_World")))

(fn `UserConstructionScript`)