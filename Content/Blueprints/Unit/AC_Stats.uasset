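; AC_Stats is a unit stats component holding base and additive stat maps keyed by source.
; AddStat writes to either map, then nested enum loops add base and additive amounts per source, category and addition type.
; Results go into AddedStats without the source key, so later sources overwrite earlier ones.
; StatsChanged broadcasts AddedStats after each rebuild, followed by a debug print, and once shortly after BeginPlay.
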(event `self.ReceiveBeginPlay`
  (`KismetSystemLibrary.Delay` 3.0)
  (`self.StatsChanged` (`self.AddedStats`)))

(fn `AddStat`
  (params (StatsFrom :type "/Game/Blueprints/Unit/Enum/E_StatsFrom Enum" :default "NewEnumerator0") (ToBase :type Boolean) (Stats :type "Map of /Game/Blueprints/InventoryEquipment/Enum/E_StatCategory Enum to /Game/Blueprints/InventoryEquipment/Struct/S_StatAmounts Structure"))
  (locals (BaseAmountsRef :type "Map of /Game/Blueprints/InventoryEquipment/Enum/E_StatAdditionType Enum to Float (double-precision)") (AdditiveAmountsRef :type "Map of /Game/Blueprints/InventoryEquipment/Enum/E_StatAdditionType Enum to Float (double-precision)") (AddedAmountsRef :type "Map of /Game/Blueprints/InventoryEquipment/Enum/E_StatAdditionType Enum to Float (double-precision)") (StatsFromRef :type "/Game/Blueprints/Unit/Enum/E_StatsFrom Enum") (StatCategoryRef :type "/Game/Blueprints/InventoryEquipment/Enum/E_StatCategory Enum") (S_StatsRef :type "Map of /Game/Blueprints/InventoryEquipment/Enum/E_StatCategory Enum to /Game/Blueprints/InventoryEquipment/Struct/S_StatAmounts Structure") (StatAditionType :type "/Game/Blueprints/InventoryEquipment/Enum/E_StatAdditionType Enum"))
  (bind _addedstats (`self.AddedStats`))
  (`BlueprintMapLibrary.Map_Add` (select `bool` (`local.ToBase`) :`false` (`self.AdditiveStats`) :`true` (`self.BaseStats`)) StatsFrom (make `/Game/Blueprints/Unit/Struct/S_Stats` Stats))
  (bind _enumvalue (foreach `/Game/Blueprints/Unit/Enum/E_StatsFrom` true)
    (:`LoopBody`
      (set `local.StatsFromRef` _enumvalue)
      (bind _enumvalue_2 (foreach `/Game/Blueprints/InventoryEquipment/Enum/E_StatCategory` true)
        (:`LoopBody`
          (set `local.StatCategoryRef` _enumvalue_2)
          (bind _enumvalue_3 (foreach `/Game/Blueprints/InventoryEquipment/Enum/E_StatAdditionType` true)
            (:`LoopBody`
              (bind _output_get (set `local.StatAditionType` _enumvalue_3))
              (`BlueprintMapLibrary.Map_Add` (`local.AddedAmountsRef`) _output_get (+ (`BlueprintMapLibrary.Map_Find` (`.Amounts_26_0915A13F4F6A65445893A8A768B38F02` (break `/Game/Blueprints/InventoryEquipment/Struct/S_StatAmounts` (`BlueprintMapLibrary.Map_Find` (`.Stats_11_11419B8A445CB92626D55E9B59AC1FFF` (break `/Game/Blueprints/Unit/Struct/S_Stats` (`BlueprintMapLibrary.Map_Find` (`self.BaseStats`) (`local.StatsFromRef`)))) (`local.StatCategoryRef`)))) (`local.StatAditionType`)) (`BlueprintMapLibrary.Map_Find` (`.Amounts_26_0915A13F4F6A65445893A8A768B38F02` (break `/Game/Blueprints/InventoryEquipment/Struct/S_StatAmounts` (`BlueprintMapLibrary.Map_Find` (`.Stats_11_11419B8A445CB92626D55E9B59AC1FFF` (break `/Game/Blueprints/Unit/Struct/S_Stats` (`BlueprintMapLibrary.Map_Find` (`self.AdditiveStats`) (`local.StatsFromRef`)))) (`local.StatCategoryRef`)))) (`local.StatAditionType`)))))
            (:`then`
              (`BlueprintMapLibrary.Map_Add` (`self.AddedStats`) (`local.StatCategoryRef`) (make `/Game/Blueprints/InventoryEquipment/Struct/S_StatAmounts` (`local.AddedAmountsRef`))))))))
    (:`then`
      (`self.StatsChanged` (`self.AddedStats`))
      ;[1 1 1] Stat Yazdırma
      (bind _keys (`BlueprintMapLibrary.Map_Keys` _addedstats))
      (for _array_element _keys
        (bind _amounts (break `/Game/Blueprints/InventoryEquipment/Struct/S_StatAmounts` (`BlueprintMapLibrary.Map_Find` _addedstats _array_element)))
        (bind _keys_2 (`BlueprintMapLibrary.Map_Keys` _amounts))
        (for _array_element_2 _keys_2
          (`KismetSystemLibrary.PrintString` (`KismetStringLibrary.Concat_StrStr` (`|GetEnumeratorNameAsString` _array_element) " - " (`|GetEnumeratorNameAsString` _array_element_2) " : " (`KismetStringLibrary.Conv_DoubleToString` (`BlueprintMapLibrary.Map_Find` _amounts _array_element_2)))))))))