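; In-game player controller that fronts the player's inventory and equipment component and applies its property changes to the controlled unit.
; Wrapper functions forward adding items, looking up item locations by ID, and moving items between inventory and equipment to that component.
; When the component reports changed properties, the controller loops over them and passes any Fire Rate amount to the BP_PlayerUnit weapon's AddFireRate, the only property handled.
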(event `self.AC_InventoryEquipment.PropertiesChanged`
  (params (Properties :type "Map of /Game/Blueprints/InventoryEquipment/Enum/E_PropertyCategory Enum to /Game/Blueprints/InventoryEquipment/Struct/S_PropertyAmounts Structure" :default _))
  (bind _keys (`BlueprintMapLibrary.Map_Keys` Properties))
  (for _array_element _keys
    (switch `/Game/Blueprints/InventoryEquipment/Enum/E_PropertyCategory` _array_element
      (:`NewEnumerator3`
        (bind _asbp_player_unit (cast `/Game/Blueprints/Player/BP_PlayerUnit` (`self.K2_GetPawn`)))
        (`/Game/Blueprints/Weapon/BP_WeaponBase.AddFireRate` (`/Game/Blueprints/Player/BP_PlayerUnit.Weapon` _asbp_player_unit) (`.PropertyNumeralAmount_8_0915A13F4F6A65445893A8A768B38F02` (break `/Game/Blueprints/InventoryEquipment/Struct/S_PropertyAmounts` (`BlueprintMapLibrary.Map_Find` Properties _array_element))))))))

(fn `AddItemToInventory`
  (params (Item :type "/Game/Blueprints/InventoryEquipment/Struct/S_Item Structure"))
  (returns (Added :type Boolean))
  (bind _added (`/Game/Blueprints/InventoryEquipment/AC_InventoryEquipment.AddItemToInventory` (`self.AC_InventoryEquipment`) Item))
  (return _added))

(fn `GetItemLocation`
  (params (ID :type Integer))
  (returns (Location :type "/Game/Blueprints/InventoryEquipment/Struct/S_ItemLocation Structure"))
  (bind _value (`/Game/Blueprints/InventoryEquipment/AC_InventoryEquipment.GetItemLocation` (`self.AC_InventoryEquipment`) ID))
  (return _value))

(fn `SendItemToEquipment`
  (params (Item :type "/Game/Blueprints/InventoryEquipment/Struct/S_Item Structure"))
  (returns (Sended :type Boolean))
  (bind _sended (`/Game/Blueprints/InventoryEquipment/AC_InventoryEquipment.SendItemToEquipment` (`self.AC_InventoryEquipment`) Item))
  (return _sended))

(fn `SendItemToInventory`
  (params (Item :type "/Game/Blueprints/InventoryEquipment/Struct/S_Item Structure"))
  (returns (Sended :type Boolean))
  (bind _sended (`/Game/Blueprints/InventoryEquipment/AC_InventoryEquipment.SendItemToInventory` (`self.AC_InventoryEquipment`) Item))
  (return _sended))

(fn `UserConstructionScript`
  (`parent.UserConstructionScript`))