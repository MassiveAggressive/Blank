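; BP_PlayerUnit is the player-controlled unit, moving on fixed world axes while turning to face an aim point.
; On BeginPlay it spawns a BP_SingleWeapon, attaches it at WeaponSpawnPoint, and sends the "LF-1" DT_Items row to its controller's inventory.
; Each tick sets only yaw toward GetHitLocation, so facing stays independent of the MoveForward and MoveRight movement input.
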(event `self.ReceiveBeginPlay`
  (`parent.ReceiveBeginPlay`)
  ;[1 1 1] SpawnWeapon
  (bind _returnvalue (`|SpawnActorFromClass` "/Game/Blueprints/Weapon/BP_SingleWeapon.BP_SingleWeapon_C" (`SceneComponent.K2_GetComponentToWorld` (`self.WeaponSpawnPoint`)) "AlwaysSpawn" "OverrideRootScale" null null))
  (bind _output_get (set `self.Weapon` _returnvalue))
  (`self.K2_AttachToComponent` _output_get (`self.WeaponSpawnPoint`) "None" "SnapToTarget" "SnapToTarget" "KeepWorld" true)
  (bind _returnvalue_2 (`|GetDataTableRow` "/Game/Blueprints/InventoryEquipment/DT_Items.DT_Items" "LF-1")
    (:`then`
      (message `/Game/Blueprints/Interface/InventoryInterface.AddItemToInventory` (`self.GetController`) _returnvalue_2))))

(event `self.ReceiveTick`
  (params (DeltaSeconds :type "Float (single-precision)"))
  (bind (_returnvalue_roll _returnvalue_pitch _returnvalue_yaw) (`KismetMathLibrary.BreakRotator` (`KismetMathLibrary.FindLookAtRotation` (`self.K2_GetActorLocation`) (`/Game/Blueprints/GeneralFunctions.GetHitLocation`))))
  (`self.K2_SetActorRotation` (`KismetMathLibrary.MakeRotator` 0.0 0.0 _returnvalue_yaw)))

(event `InputAxis|MoveForward`
  (params (AxisValue :type "Float (single-precision)"))
  (`self.AddMovementInput` (1.0 0.0 0.0) AxisValue))

(event `InputAxis|MoveRight`
  (params (AxisValue :type "Float (single-precision)"))
  (`self.AddMovementInput` (0.0 1.0 0.0) AxisValue))

(fn `UserConstructionScript`
  (`parent.UserConstructionScript`))