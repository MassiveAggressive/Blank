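; BP_CollectableItem is a world item actor that can be picked up into an inventory.
; On BeginPlay it looks up its data table row, passes it to its W_CollectableItemInfo widget and stores it as the Item.
; On Interact it sends the Item to the interactor's controller through BPI_InventoryEquipment, then destroys itself without checking whether the add succeeded.
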(event `self.ReceiveBeginPlay`
  (bind (_datatable _rowname) (break `DataTableRowHandle` (`self.ItemDataTableRow`)))
  (bind _returnvalue (`|GetDataTableRow` _datatable _rowname)
    (:`then`
      (bind _asw_collectable_item_info (cast `/Game/Blueprints/InventoryEquipment/Widget/W_CollectableItemInfo` (`WidgetComponent.GetWidget` (`self.Widget`))))
      (`/Game/Blueprints/InventoryEquipment/Widget/W_CollectableItemInfo.SetItem` _asw_collectable_item_info _returnvalue)
      (set `self.Item` _returnvalue))))

(event `/Game/Blueprints/Interact/Interface/BPI_Interact.Interact`
  (params (Interactor :type "Pawn Object Reference"))
  (bind _returnvalue (`Pawn.GetController` Interactor))
  (if (`KismetSystemLibrary.DoesImplementInterface` _returnvalue "/Game/Blueprints/InventoryEquipment/Interface/BPI_InventoryEquipment.BPI_InventoryEquipment_C")
    (message `/Game/Blueprints/InventoryEquipment/Interface/BPI_InventoryEquipment.AddItemToInventory` _returnvalue (`self.Item`))
    (`self.K2_DestroyActor`)))

(fn `UserConstructionScript`
  (`parent.UserConstructionScript`))