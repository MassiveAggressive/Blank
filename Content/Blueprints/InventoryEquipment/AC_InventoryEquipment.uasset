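; Inventory and equipment component that stores items grouped by item type and moves them between the two.
; Type-keyed maps of array structs are written back after each edit, with equipment capped by per-type slot sizes.
; An ID map records each inventory item's type and index for removal, but indices are not refreshed after removals.
; Dispatchers announce additions and removals; the inventory widget creation is left unconnected.
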(event `self.ReceiveBeginPlay`)

(fn `AddItemToEquipment`
  (params (Item :type "/Game/Blueprints/InventoryEquipment/Struct/S_Item Structure"))
  (returns (Added :type Boolean))
  (locals (ItemTypeRef :type "/Game/Blueprints/InventoryEquipment/Enum/E_ItemType Enum") (ItemArrayRef :type "Array of /Game/Blueprints/InventoryEquipment/Struct/S_Item Structure"))
  (bind _output_get (set `local.ItemTypeRef` (`.ItemType_35_B85020CC4326255BF9CA7986369ED08C` (break `/Game/Blueprints/InventoryEquipment/Struct/S_Item` Item))))
  (bind _isthere (`self.IsThereEmptySlotInEquipment` _output_get))
  (if _isthere
    (bind _output_get_2 (set `local.ItemArrayRef` (`.Array_3_54825DA340DDAE3ADDAE89ABB7425895` (break `/Game/Blueprints/InventoryEquipment/Struct/S_ItemArray` (`BlueprintMapLibrary.Map_Find` (`self.EquipmentArray`) (`local.ItemTypeRef`))))))
    (`KismetArrayLibrary.Array_Add` _output_get_2 (`local.Item`))
    (`BlueprintMapLibrary.Map_Add` (`self.EquipmentArray`) (`local.ItemTypeRef`) (make `/Game/Blueprints/InventoryEquipment/Struct/S_ItemArray` (`local.ItemArrayRef`)))
    (`KismetArrayLibrary.Array_Clear` (`local.ItemArrayRef`))
    (`self.ItemAddedToEquipment` (`local.Item`))
    (return true)
    (else
      (return false))))

(fn `AddItemToInventory`
  (params (Item :type "/Game/Blueprints/InventoryEquipment/Struct/S_Item Structure"))
  (returns (Added :type Boolean))
  (locals (ItemTypeRef :type "/Game/Blueprints/InventoryEquipment/Enum/E_ItemType Enum") (ItemArrayRef :type "Array of /Game/Blueprints/InventoryEquipment/Struct/S_Item Structure"))
  (bind ((`ID_34_480AFE364D7F3357C84857B4B302F81E` _id) (`ItemType_35_B85020CC4326255BF9CA7986369ED08C` _itemtype)) (break `/Game/Blueprints/InventoryEquipment/Struct/S_Item` (`local.Item`)))
  (set `local.ItemTypeRef` (`.ItemType_35_B85020CC4326255BF9CA7986369ED08C` (break `/Game/Blueprints/InventoryEquipment/Struct/S_Item` Item)))
  (bind _output_get (set `local.ItemArrayRef` (`.Array_3_54825DA340DDAE3ADDAE89ABB7425895` (break `/Game/Blueprints/InventoryEquipment/Struct/S_ItemArray` (`BlueprintMapLibrary.Map_Find` (`self.InventoryArray`) (`local.ItemTypeRef`))))))
  (bind _returnvalue (`KismetArrayLibrary.Array_Add` _output_get (`local.Item`)))
  (`BlueprintMapLibrary.Map_Add` (`self.InventoryArray`) (`local.ItemTypeRef`) (make `/Game/Blueprints/InventoryEquipment/Struct/S_ItemArray` (`local.ItemArrayRef`)))
  (`KismetArrayLibrary.Array_Clear` (`local.ItemArrayRef`))
  (`BlueprintMapLibrary.Map_Add` (`self.InventoryIDs`) _id (make `/Game/Blueprints/InventoryEquipment/Struct/S_ItemLocationInInventory` _itemtype _returnvalue))
  (`self.ItemAddedToInventory` (`local.Item`))
  (return true))

(fn `IsThereEmptySlotInEquipment`
  (params (ItemType :type "/Game/Blueprints/InventoryEquipment/Enum/E_ItemType Enum" :default "NewEnumerator0"))
  (returns (IsThere :type Boolean))
  (return (< (`KismetArrayLibrary.Array_Length` (`.Array_3_54825DA340DDAE3ADDAE89ABB7425895` (break `/Game/Blueprints/InventoryEquipment/Struct/S_ItemArray` (`BlueprintMapLibrary.Map_Find` (`self.EquipmentArray`) ItemType)))) (`BlueprintMapLibrary.Map_Find` (`self.EquipmentSlotsSizes`) ItemType))))

(fn `SendItemToEquipment`
  (params (Item :type "/Game/Blueprints/InventoryEquipment/Struct/S_Item Structure"))
  (locals (ItemArrayRef :type "Array of /Game/Blueprints/InventoryEquipment/Struct/S_Item Structure"))
  (bind (_itemtype _index) (break `/Game/Blueprints/InventoryEquipment/Struct/S_ItemLocationInInventory` (`BlueprintMapLibrary.Map_Find` (`self.InventoryIDs`) (`.ID_34_480AFE364D7F3357C84857B4B302F81E` (break `/Game/Blueprints/InventoryEquipment/Struct/S_Item` (`local.Item`))))))
  (bind _added (`self.AddItemToEquipment` Item))
  (if _added
    (bind _output_get (set `local.ItemArrayRef` (`.Array_3_54825DA340DDAE3ADDAE89ABB7425895` (break `/Game/Blueprints/InventoryEquipment/Struct/S_ItemArray` (`BlueprintMapLibrary.Map_Find` (`self.InventoryArray`) _itemtype)))))
    (`KismetArrayLibrary.Array_Remove` _output_get _index)
    (`BlueprintMapLibrary.Map_Add` (`self.InventoryArray`) (`.ItemType_35_B85020CC4326255BF9CA7986369ED08C` (break `/Game/Blueprints/InventoryEquipment/Struct/S_Item` (`local.Item`))) (make `/Game/Blueprints/InventoryEquipment/Struct/S_ItemArray` (`local.ItemArrayRef`)))
    (`BlueprintMapLibrary.Map_Remove` (`self.InventoryIDs`) (`.ID_34_480AFE364D7F3357C84857B4B302F81E` (break `/Game/Blueprints/InventoryEquipment/Struct/S_Item` (`local.Item`))))
    (`self.ItemRemovedFromInventory` (`local.Item`))))

(fn `SendItemToInventory`
  (params (Item :type "/Game/Blueprints/InventoryEquipment/Struct/S_Item Structure"))
  (locals (ItemArrayRef :type "Array of /Game/Blueprints/InventoryEquipment/Struct/S_Item Structure"))
  (bind _added (`self.AddItemToInventory` Item))
  (if _added
    (bind _output_get (set `local.ItemArrayRef` (`.Array_3_54825DA340DDAE3ADDAE89ABB7425895` (break `/Game/Blueprints/InventoryEquipment/Struct/S_ItemArray` (`BlueprintMapLibrary.Map_Find` (`self.EquipmentArray`) (`.ItemType_35_B85020CC4326255BF9CA7986369ED08C` (break `/Game/Blueprints/InventoryEquipment/Struct/S_Item` (`local.Item`))))))))
    (`KismetArrayLibrary.Array_Remove` _output_get (`KismetArrayLibrary.Array_Find` _output_get (`local.Item`)))
    (`BlueprintMapLibrary.Map_Add` (`self.EquipmentArray`) (`.ItemType_35_B85020CC4326255BF9CA7986369ED08C` (break `/Game/Blueprints/InventoryEquipment/Struct/S_Item` (`local.Item`))) (make `/Game/Blueprints/InventoryEquipment/Struct/S_ItemArray` (`local.ItemArrayRef`)))
    (`self.ItemRemovedFromEquipment` (`local.Item`))))