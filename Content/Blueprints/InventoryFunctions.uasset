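; Blueprint function library of inventory helpers that add items with unique integer IDs to the player's inventory.
; GetInventoryEquipmentComp returns the inventory equipment component from player 0's BP_InGamePlayerController.
; CreateANewID takes the highest key in that component's InventoryIDs map plus one.
; AddItem stamps this ID on the item struct, passes it to AddItemToInventory and prints the ID.
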(fn `AddItem`
  (params (Item :type "/Game/Blueprints/InventoryEquipment/Struct/S_Item Structure") (__WorldContext :type "Object Object Reference"))
  (locals (ItemRef :type "/Game/Blueprints/InventoryEquipment/Struct/S_Item Structure"))
  (set `local.ItemRef` Item)
  (bind _id (`self.CreateANewID` null))
  (bind _structout (setmembers `/Game/Blueprints/InventoryEquipment/Struct/S_Item` :`StructRef` (`local.ItemRef`) :`ID` _id))
  (`/Game/Blueprints/InventoryEquipment/AC_InventoryEquipment.AddItemToInventory` (`self.GetInventoryEquipmentComp` null) _structout)
  (`KismetSystemLibrary.PrintString` null (`KismetStringLibrary.Conv_IntToString` (`.ID_34_480AFE364D7F3357C84857B4B302F81E` (break `/Game/Blueprints/InventoryEquipment/Struct/S_Item` _structout)))))

(fn `CreateANewID`
  (params (__WorldContext :type "Object Object Reference"))
  (returns (ID :type Integer))
  (locals (IDArrayRef :type "Array of Integer") (IDRef :type Integer :default 0))
  (bind _keys (`BlueprintMapLibrary.Map_Keys` (`/Game/Blueprints/InventoryEquipment/AC_InventoryEquipment.InventoryIDs` (`self.GetInventoryEquipmentComp` null))))
  (bind _output_get (set `local.IDArrayRef` _keys))
  (bind _output_get_2 (set `local.IDRef` (+ (`.MaxValue` (`KismetMathLibrary.MaxOfIntArray` _output_get)) 1)))
  (return _output_get_2))

(fn `GetInventoryEquipmentComp`
  (params (__WorldContext :type "Object Object Reference"))
  (returns (Component :type "/Game/Blueprints/InventoryEquipment/AC_InventoryEquipment Object Reference"))
  (bind _asbp_in_game_player_controller (cast `/Game/Blueprints/Player/BP_InGamePlayerController` (`GameplayStatics.GetPlayerController` null)))
  (return (`/Game/Blueprints/Player/BP_InGamePlayerController.AC_InventoryEquipment` _asbp_in_game_player_controller)))