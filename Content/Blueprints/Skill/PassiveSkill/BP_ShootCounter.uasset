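; BP_ShootCounter is a passive skill that turns every few regular weapon shots into a rapid burst.
; CountShoot tallies shots not affected by the skill, and on the fifth it pauses shooting and starts a looping timer at four times the weapon's fire rate.
; CallShoot fires four flagged shots, then clears the timer and resumes normal shooting.
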(fn `ApplySkill`
  (`parent.ApplySkill`))

(fn `CallShoot`
  (`/Game/Blueprints/Weapon/BP_WeaponBase.Shoot` (`self.AffectedWeapon`) true)
  (bind _result (`/Engine/EditorBlueprintResources/StandardMacros.IncrementInt` (`self.ShootCountCount`))
    (:`  `
      (if (== _result 4)
        (`/Game/Blueprints/Weapon/BP_WeaponBase.StartShooting` (`self.AffectedWeapon`))
        (`KismetSystemLibrary.K2_ClearAndInvalidateTimerHandle` (`self.CallShootTimer`))
        (set `self.ShootCountCount` 0)))))

(fn `CountShoot`
  (params (AffectedBySkill :type Boolean))
  (if (not AffectedBySkill)
    (bind _result (`/Engine/EditorBlueprintResources/StandardMacros.IncrementInt` (`self.ShootCount`))
      (:`  `
        (if (== _result 5)
          (`/Game/Blueprints/Weapon/BP_WeaponBase.StopShooting` (`self.AffectedWeapon`))
          (bind _returnvalue (`KismetSystemLibrary.K2_SetTimerDelegate` (`|CreateDelegate` :!event `CallShoot`) (/ (/ 1.0 (`/Game/Blueprints/Weapon/BP_WeaponBase.FireRate` (`self.AffectedWeapon`))) 4.0) true))
          (set `self.CallShootTimer` _returnvalue)
          (set `self.ShootCount` 0))))))