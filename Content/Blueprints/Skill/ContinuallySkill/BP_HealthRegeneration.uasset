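; BP_HealthRegeneration is a continual skill that restores health to its affected object.
; When applied, it reads RegenerationAmount from the skill data table row matching the skill level, and calls the parent ApplySkill only if that row is found.
; Each run of ContinuallyFunction calls the parent version, then sends that amount through BPI_HealthInterface's AddHealthMessage if the affected object implements the interface.
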(fn `ApplySkill`
  (bind ((`Level_20_86ED8EE245A0123F80827A883D93731F` _level) (`SkillDataTable_24_AB22FA964BE2859BA8500BB7569B1342` _skilldatatable)) (break `/Game/Blueprints/Skill/Struct/S_Skill` (`self.SkillProperties`)))
  (bind _returnvalue (`|GetDataTableRow` _skilldatatable (`KismetStringLibrary.Conv_StringToName` (`KismetStringLibrary.Conv_IntToString` _level)))
    (:`then`
      (set `self.RegenerationAmount` (`.RegenerationAmount_2_DD33E2E1418CD6BD083E3DA11C32083E` (break `/Game/Blueprints/Skill/ContinuallySkill/S_HealthRegenerationSkill` _returnvalue)))
      (`parent.ApplySkill`))))

(fn `ContinuallyFunction`
  (`parent.ContinuallyFunction`)
  (if (`KismetSystemLibrary.DoesImplementInterface` (`self.AffectedObject`) "/Game/Blueprints/Health/BPI_HealthInterface.BPI_HealthInterface_C")
    (message `/Game/Blueprints/Health/BPI_HealthInterface.AddHealth` (`self.AffectedObject`) "NewEnumerator0" (`self.RegenerationAmount`))))