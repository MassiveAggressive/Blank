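; Base skill Blueprint for continuous skills that repeat an effect at a fixed rate once applied.
; ApplySkill runs the parent logic, then reads the Rate from the skill's data table row named after its level.
; That rate sets a looping timer, with a stored handle, that calls ContinuallyFunction every 1/Rate seconds.
; ContinuallyFunction is empty here, serving as the hook for child skills.
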(fn `ApplySkill`
  (bind ((`Level_20_86ED8EE245A0123F80827A883D93731F` _level) (`SkillDataTable_24_AB22FA964BE2859BA8500BB7569B1342` _skilldatatable)) (break `/Game/Blueprints/Skill/Struct/S_Skill` (`self.SkillProperties`)))
  (`parent.ApplySkill`)
  (bind _returnvalue (`|GetDataTableRow` _skilldatatable (`KismetStringLibrary.Conv_StringToName` (`KismetStringLibrary.Conv_IntToString` _level)))
    (:`then`
      (bind _rate (break `/Game/Blueprints/Skill/ContinuallySkill/S_ContinuallySkill` _returnvalue))
      (set `self.Rate` _rate)
      (bind _returnvalue_2 (`KismetSystemLibrary.K2_SetTimer` self "ContinuallyFunction" (/ 1.0 _rate) true))
      (set `self.ContinuallyFunctionTimer` _returnvalue_2))))

(fn `ContinuallyFunction`)