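; BP_SkillBase is the base Blueprint for a skill that tracks its own state and category.
; It stores a SkillState enum with a getter and setter, and ApplySkill sets it to a fixed enum value.
; RequestAcquire fires the OnAcquireRequest dispatcher, passing the category from SkillProperties and itself, so listeners handle acquisition.
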(fn `ApplySkill`
  (set `self.SkillState` "NewEnumerator2"))

(fn `GetState`
  (returns (SkillState :type "/Game/Blueprints/Skill/Enum/E_SkillState Enum"))
  (return (`self.SkillState`)))

(fn `RequestAcquire`
  (`self.OnAcquireRequest` (`.SkillCategory_7_C9DCE8974261B07E59F5FC9C210D293B` (break `/Game/Blueprints/Skill/Struct/S_Skill` (`self.SkillProperties`))) self))

(fn `SetState`
  (params (SkillState :type "/Game/Blueprints/Skill/Enum/E_SkillState Enum" :default "NewEnumerator0"))
  (set `self.SkillState` SkillState))