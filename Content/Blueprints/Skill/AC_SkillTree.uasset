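; Skill tree component on a Controller that manages skill objects per category and spends skill points to apply them.
; AddSkill constructs each skill from its struct, binds its acquire request, files it in a category map, and changes the first one's state.
; OnSkillAcquire applies the skill, then advances the next in that category, signalling acquisition only if one exists.
; Widget creation and DT_Skill loading are unwired; BeginPlay only caches the pawn.
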(event `self.ReceiveBeginPlay`
  (set `self.OwnerActor` (`Controller.K2_GetPawn` (cast `Controller` (`self.GetOwner`) :!pure true))))

(fn `AddSkill`
  (params (Skill :type "/Game/Blueprints/Skill/Struct/S_Skill Structure"))
  (locals (S_SkillRef :type "/Game/Blueprints/Skill/Struct/S_Skill Structure") (SkillRef :type "/Game/Blueprints/Skill/BP_SkillBase Object Reference") (SkillArrayRef :type "Array of /Game/Blueprints/Skill/BP_SkillBase Object Reference") (SkillCategoryRef :type "/Game/Blueprints/Skill/Enum/E_SkillCategory Enum") (SkillAddedNum :type Integer :default 0))
  (bind _output_get (set `local.S_SkillRef` Skill))
  (bind (_name _description _skillcategory _skill) (break `/Game/Blueprints/Skill/Struct/S_Skill` _output_get))
  (set `local.SkillCategoryRef` _skillcategory)
  (bind _returnvalue (`|GenericCreateObject` _skill self (`local.S_SkillRef`)))
  (bind _output_get_2 (set `local.SkillRef` _returnvalue))
  (add `/Game/Blueprints/Skill/BP_SkillBase.OnAcquireRequest` _output_get_2 (`|CreateDelegate` :!event `OnSkillAcquire`))
  (bind _output_get_3 (set `local.SkillArrayRef` (`.Array_4_19E32EA14D2EBCDE55D091BD3502F861` (break `/Game/Blueprints/Skill/Struct/S_SkillArray` (`BlueprintMapLibrary.Map_Find` (`self.SkillArray`) (`local.SkillCategoryRef`))))))
  (bind _returnvalue_2 (`KismetArrayLibrary.Array_Add` _output_get_3 (`local.SkillRef`)))
  (set `local.SkillAddedNum` _returnvalue_2)
  (`BlueprintMapLibrary.Map_Add` (`self.SkillArray`) (`local.SkillCategoryRef`) (make `/Game/Blueprints/Skill/Struct/S_SkillArray` (`local.SkillArrayRef`)))
  (`KismetArrayLibrary.Array_Clear` (`local.SkillArrayRef`))
  (if (== (`local.SkillAddedNum`) 0)
    (`/Game/Blueprints/Skill/BP_SkillBase.SetState` (`local.SkillRef`) "NewEnumerator1"))
  (`self.SkillAdded` (`local.SkillCategoryRef`) (`local.SkillRef`)))

(fn `OnSkillAcquire`
  (params (SkillCategory :type "/Game/Blueprints/Skill/Enum/E_SkillCategory Enum" :default "NewEnumerator0") (Skill :type "/Game/Blueprints/Skill/BP_SkillBase Object Reference"))
  (locals (SkillArrayRef :type "Array of /Game/Blueprints/Skill/BP_SkillBase Object Reference"))
  (if (> (`self.SkillPoints`) 0)
    (`/Game/Blueprints/Skill/BP_SkillBase.ApplySkill` Skill)
    (`/Engine/EditorBlueprintResources/StandardMacros.DecrementInt` (`self.SkillPoints`)
      (:`  `
        (bind _output_get (set `local.SkillArrayRef` (`.Array_4_19E32EA14D2EBCDE55D091BD3502F861` (break `/Game/Blueprints/Skill/Struct/S_SkillArray` (`BlueprintMapLibrary.Map_Find` (`self.SkillArray`) (`local.SkillCategory`))))))
        (bind _returnvalue (+ (`KismetArrayLibrary.Array_Find` _output_get (`local.Skill`)) 1))
        (if (`KismetArrayLibrary.Array_IsValidIndex` _output_get _returnvalue)
          (`/Game/Blueprints/Skill/BP_SkillBase.SetState` (`|GetArrayItem` (`local.SkillArrayRef`) _returnvalue) "NewEnumerator1")
          (`self.SkillAcquired` (`local.SkillCategory`) (`local.Skill`)))))))