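; AC_HealthComponent is a component that tracks an actor's health, starting at MaxHealth on BeginPlay.
; AddHealth adds or subtracts a value based on a Regeneration or Damage type, clamps it between zero and MaxHealth, and fires OnDestroy at zero.
; AddMaxHealth and SetMaxHealth adjust the cap without changing current health.
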(event `self.ReceiveBeginPlay`
  (set `self.Health` (`self.MaxHealth`)))

(fn `AddHealth`
  (params (AddHealthType :type "/Game/Blueprints/Health/E_AddHealthType Enum" :default "NewEnumerator0") (Value :type "Float (double-precision)"))
  (bind _output_get (set `self.Health` (`KismetMathLibrary.FClamp` (+ (`self.Health`) (* Value (select `/Game/Blueprints/Health/E_AddHealthType` AddHealthType :`NewEnumerator0` 1.0 :`NewEnumerator1` -1.0 :!type "Float (single-precision)"))) 0.0 (`self.MaxHealth`))))
  (if (== _output_get 0.0)
    (`self.OnDestroy`)))

(fn `AddMaxHealth`
  (params (Value :type "Float (double-precision)"))
  (set `self.MaxHealth` (+ (`self.MaxHealth`) Value)))

(fn `SetMaxHealth`
  (params (Value :type "Float (double-precision)"))
  (set `self.MaxHealth` Value))