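; BP_InteractBase is a base actor for interactables, providing a configurable overlap volume.
; The Construction Script adds a sphere or box component based on CollisionType, sized by Radius or Extent, and sets the sphere visible in game.
; It binds the component's begin and end overlap events to BeginOverlap and EndOverlap, which are empty here, as are the event graph's events.
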(fn `BeginOverlap`
  (params (OverlappedComponent :type "PrimitiveComponent Object Reference") (OtherActor :type "Actor Object Reference") (OtherComp :type "PrimitiveComponent Object Reference") (OtherBodyIndex :type Integer) (bFromSweep :type Boolean) (SweepResult :type "HitResult Structure (by ref)")))

(fn `EndOverlap`
  (params (OverlappedComponent :type "PrimitiveComponent Object Reference") (OtherActor :type "Actor Object Reference") (OtherComp :type "PrimitiveComponent Object Reference") (OtherBodyIndex :type Integer)))

(fn `UserConstructionScript`
  (switch `/Game/Blueprints/Interact/Enum/E_CollisionType` (`self.CollisionType`)
    (:`NewEnumerator0`
      (bind _returnvalue (`AddComponent|NODE_AddSphereComponent-0`))
      (`SphereComponent.SetSphereRadius` _returnvalue (`self.Radius`) true))
    (:`NewEnumerator1`
      (bind _returnvalue_2 (`AddComponent|NODE_AddBoxComponent-0`))
      (`BoxComponent.SetBoxExtent` _returnvalue_2 (`self.Extent`) true)))
  (add `PrimitiveComponent.OnComponentBeginOverlap` _returnvalue_2 (`|CreateDelegate` :!event `BeginOverlap`))
  (add `PrimitiveComponent.OnComponentBeginOverlap` _returnvalue (`|CreateDelegate` :!event `BeginOverlap`))
  (add `PrimitiveComponent.OnComponentEndOverlap` _returnvalue_2 (`|CreateDelegate` :!event `EndOverlap`))
  (add `PrimitiveComponent.OnComponentEndOverlap` _returnvalue (`|CreateDelegate` :!event `EndOverlap`))
  (`SceneComponent.SetHiddenInGame` _returnvalue false false))